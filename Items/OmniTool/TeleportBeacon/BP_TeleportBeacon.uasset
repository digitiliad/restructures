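; BP_TeleportBeacon is a temporary beacon placed for the OmniTool's personal teleporter that destroys itself after a configurable lifespan.
; On BeginPlay, after a short delay, the server registers it in the "SplusTeleporterBeacon" custom actor list and removes its inventory component.
; A timer read from game mode config triggers DestroySelfEvent, which unregisters the beacon on authority and destroys the actor.
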(event `self.ReceiveBeginPlay`
  (`KismetSystemLibrary.Delay` 0.2)
  (`/Engine/EditorBlueprintResources/ActorMacros.Switch Has Authority`
    (:`Authority`
      (`/Game/Mods/StructuresPlusMod/_Scripts/ActorFunctions.SP_AddToCustomActorList` self "SplusTeleporterBeacon")
      (`ActorComponent.K2_DestroyComponent` (`self.MyInventoryComponent`))
      (bind _value (`/Game/Mods/StructuresPlusMod/_Scripts/ConfigFunctions.SP_GetConfig_-_Float` (`GameplayStatics.GetGameMode`) "PersonalTeleporterBeaconLifespanInSeconds" 300.0 10.0 3600.0))
      (`KismetSystemLibrary.K2_SetTimerDelegate` (delegate `DestroySelfEvent`) _value))))

(event `DestroySelfEvent`
  (`|ExecutionSequence`
    (:`then_0`
      (`/Engine/EditorBlueprintResources/ActorMacros.Switch Has Authority`
        (:`Authority`
          (bind _returnvalue (`VictoryCore.GetCustomActorList` (`self.K2_GetWorld`) "SplusTeleporterBeacon"))
          (`/Engine/EditorBlueprintResources/StandardMacros.IsValid` _returnvalue
            (:`Is Valid`
              (`KismetArrayLibrary.Array_RemoveItem` (`CustomActorList.ActorList` _returnvalue) self))))))
    (:`then_1`
      (`self.K2_DestroyActor`))))

(fn `UserConstructionScript`
  (`parent.UserConstructionScript`))