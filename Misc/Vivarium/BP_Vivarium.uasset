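; BP_Vivarium is a placeable structure that holds stored dino data and releases it back into the world as live dinos.
; Players with structure access get a "Remove a Dino" multi-use entry, which checks the tame cap before spawning the first stored dino above the structure.
; On destruction or pickup, the server releases stored dinos in a bounded loop while under the tame cap.
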(fn `BPGetMultiUseEntries`
  (params (ForPC :type "PlayerController Object Reference") (MultiUseEntries :type "Array of Actor.MultiUseEntry Structure (by ref)"))
  (returns (ReturnValue :type "Array of Actor.MultiUseEntry Structure"))
  (bind _hasdinos (`self.HasDinos`))
  (bind _entriesout (`/Game/Mods/StructuresPlusMod/_Scripts/MultiUseMenuFunctions.SP_Update_Multi_Use_Menu` ForPC MultiUseEntries self))
  (`|ExecutionSequence`
    (:`then_0`
      (bind _returnvalue (`self.AllowStructureAccess` ForPC))
      (if _returnvalue
        (`KismetArrayLibrary.Array_Add` _entriesout (make `Actor.MultiUseEntry` :`UseString` "Remove a Dino" :`UseIndex` 9900 :`Priority` (`KismetMathLibrary.SelectInt` 5000 -5000 _hasdinos) :`bHideFromUI` (not _hasdinos) :`bDisplayOnInventoryUI` _hasdinos))))
    (:`then_1`
      (return _entriesout))))

(fn `BPOnStructurePickup`
  (params (PlayerController :type "PlayerController Object Reference") (ItemType :type "PrimalItem Class Reference") (NewlyPickedUpItem :type "PrimalItem Object Reference") (bIsQuickPickup :type Boolean))
  (`/Engine/EditorBlueprintResources/ActorMacros.Switch Has Authority`
    (:`Authority`
      (`/Game/Mods/StructuresPlusMod/_Macros/UtilityMacros.SP_While` (and (`self.IsUnderTameCap`) (> (`KismetArrayLibrary.Array_Length` (`self.DinoDataList`)) 0)) 11
        (:`Loop Body`
          (`self.RemoveDino` null))))))

(fn `BPTryMultiUse`
  (params (ForPC :type "PlayerController Object Reference") (UseIndex :type Integer))
  (returns (ReturnValue :type Boolean))
  (`|ExecutionSequence`
    (:`then_0`
      (if (== UseIndex 601)
        (set `self.IsUnlocked` (not (`self.bIsLocked`)))
        (elif (== UseIndex 9900)
          (if (`self.IsUnderTameCap`)
            (`self.RemoveDino` ForPC)
            (else
              (`StructuresPlus.SP_MessageClient` ForPC "You have reached your tame limit." "Error"))))))
    (:`then_1`
      (return true))))

(fn `IsUnderTameCap`
  (returns (IsUnder :type Boolean))
  (bind _asshootergamestate (cast `ShooterGameState` (`GameplayStatics.GetGameState`) :!pure true))
  (bind _returnvalue (`ShooterGameMode.AllowTaming` (cast `ShooterGameMode` (`GameplayStatics.GetGameMode`) :!pure true) (`self.TargetingTeam`)))
  (return (or _returnvalue (and (`ShooterGameState.bServerPVE` _asshootergamestate) (< (`ShooterGameState.NumTamedDinos` _asshootergamestate) (`ShooterGameState.MaxTamedDinos` _asshootergamestate))))))

(fn `ReceiveBeginPlay`
  (`parent.ReceiveBeginPlay`)
  (if (and (`KismetSystemLibrary.IsServer`) (not (`self.bIsPreviewStructure`)))
    (set `self.bIsLocked` (not (`self.IsUnlocked`)) true)
    (set `self.HasDinos` (> (`KismetArrayLibrary.Array_Length` (`self.DinoDataList`)) 0) true)))

(fn `ReceiveDestroyed`
  (`/Engine/EditorBlueprintResources/ActorMacros.Switch Has Authority`
    (:`Authority`
      (`/Game/Mods/StructuresPlusMod/_Macros/UtilityMacros.SP_While` (and (`self.IsUnderTameCap`) (> (`KismetArrayLibrary.Array_Length` (`self.DinoDataList`)) 0)) 11
        (:`Loop Body`
          (`self.RemoveDino` null))))))

(fn `RemoveDino`
  (params (PC :type "PlayerController Object Reference"))
  (bind _dinodatalist (`self.DinoDataList`))
  (bind _dinodatalist_2 (`self.DinoDataList`))
  (if (`KismetArrayLibrary.Array_IsValidIndex` _dinodatalist_2)
    (bind _returnvalue (`PrimalDinoCharacter.SpawnFromDinoData` (`KismetArrayLibrary.Array_Get` _dinodatalist_2) (`self.K2_GetWorld`) (+ (.location (`self.GetTransform`)) (0.0 0.0 300.0)) (.rotation (`self.GetTransform`)) (`self.TargetingTeam`) true))
    (`/Engine/EditorBlueprintResources/StandardMacros.IsValid` _returnvalue
      (:`Is Valid`
        (bind _mycharacterstatuscomponent (`PrimalCharacter.MyCharacterStatusComponent` _returnvalue))
        (`PrimalCharacterStatusComponent.RescaleAllStats` _mycharacterstatuscomponent)
        (`PrimalCharacterStatusComponent.ServerSyncReplicatedValues` _mycharacterstatuscomponent)
        (`KismetArrayLibrary.Array_Remove` _dinodatalist)
        (set `self.HasDinos` (> (`KismetArrayLibrary.Array_Length` _dinodatalist) 0) true)
        (`StructuresPlus.SP_MessageClient` PC "Dino Removed!" "Default"))
      (:`Is Not Valid`
        (`StructuresPlus.SP_MessageClient` PC "Failed to spawn dino in world." "Error")))))

(fn `UserConstructionScript`
  (`parent.UserConstructionScript`))