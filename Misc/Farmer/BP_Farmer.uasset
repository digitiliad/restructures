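; Farmer structure that automatically collects fertilizer from beetles and compost bins and distributes it to crops.
; On BeginPlay the authority loads slot count and range from game config and flags fertilizer in the inherited collect and distribute data.
; While activated, DoScan re-arms its own timer, cycling through beetle collection, compost bin collection and crop distribution one step per tick.
; Same-team players get multi-use entries to toggle collection and distribution separately.
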(fn `BPGetMultiUseEntries`
  (params (ForPC :type "PlayerController Object Reference") (MultiUseEntries :type "Array of Actor.MultiUseEntry Structure (by ref)"))
  (returns (ReturnValue :type "Array of Actor.MultiUseEntry Structure"))
  (bind _returnvalue (`parent.BPGetMultiUseEntries` ForPC MultiUseEntries))
  (`|ExecutionSequence`
    (:`then_0`
      (if (== (`Actor.TargetingTeam` ForPC) (`self.TargetingTeam`))
        (`KismetArrayLibrary.Array_Add` _returnvalue (make `Actor.MultiUseEntry` :`UseString` (`KismetMathLibrary.SelectString` "Enable Fertilizer Collection" "Disable Fertilizer Collection" (`self.DisableCollection`)) :`UseIndex` 9003 :`Priority` -1005 :`bDisplayOnInventoryUISecondary` true))
        (`KismetArrayLibrary.Array_Add` _returnvalue (make `Actor.MultiUseEntry` :`UseString` (`KismetMathLibrary.SelectString` "Enable Fertilizer Distribution" "Disable Fertilizer Distribution" (`self.DisableFertDistribution`)) :`UseIndex` 9004 :`Priority` -1006 :`bDisplayOnInventoryUITertiary` true))))
    (:`then_1`
      (return _returnvalue))))

(fn `BPTryMultiUse`
  (params (ForPC :type "PlayerController Object Reference") (UseIndex :type Integer))
  (returns (ReturnValue :type Boolean))
  (`parent.BPTryMultiUse` ForPC UseIndex)
  (`|ExecutionSequence`
    (:`then_0`
      (switch `int` UseIndex
        (:`9003`
          (set `self.DisableCollection` (not (`self.DisableCollection`)) true))
        (:`9004`
          (set `self.DisableFertDistribution` (not (`self.DisableFertDistribution`)) true))))
    (:`then_1`
      (return true))))

(fn `DoScan`
  (bind _returnvalue (not (`self.DisableCollection`)))
  (bind _returnvalue_2 (+ (`self.SecondaryScanIndex`) 1))
  (if (`self.bContainerActivated`)
    (`PrimalInventoryComponent.InventoryRefresh` (`self.MyInventoryComponent`))
    (`|ExecutionSequence`
      (:`then_0`
        (switch `int` (`self.SecondaryScanIndex`)
          (:`0`
            (if _returnvalue
              (`self.Collect_-_Beetles`)))
          (:`1`
            (if _returnvalue
              (`self.Collect_-_CompostBins`)))
          (:`2`
            (if (not (`self.DisableFertDistribution`))
              (`self.Distribute_-_Crops`)))))
      (:`then_1`
        (set `self.SecondaryScanIndex` (`KismetMathLibrary.SelectInt` 0 _returnvalue_2 (> _returnvalue_2 2)))
        (`KismetSystemLibrary.K2_SetTimer` null "DoScan" (`self.GetScanInterval`))))))

(fn `ReceiveBeginPlay`
  (bind _returnvalue (`GameplayStatics.GetGameMode`))
  (`parent.ReceiveBeginPlay`)
  (if (not (`self.bIsPreviewStructure`))
    (`/Engine/EditorBlueprintResources/ActorMacros.Switch Has Authority`
      (:`Authority`
        (`|ExecutionSequence`
          (:`then_0`
            (bind _value (`/Game/Mods/StructuresPlusMod/_Scripts/ConfigFunctions.SP_GetConfigSetting_-_InventorySize` _returnvalue "FarmerSlotCount" 300))
            (set `self.InvSlotOverride` _value true))
          (:`then_1`
            (bind _value_2 (`/Game/Mods/StructuresPlusMod/_Scripts/ConfigFunctions.SP_GetConfig_-_Int` _returnvalue "FarmerRangeInFoundations" 25 1 100))
            (set `self.ScanRadius` (* _value_2 300.0) true))
          (:`then_2`
            (setmembers `/Game/Mods/StructuresPlusMod/_Structs/SP_ItemCollectorCollectData` :`StructRef` (`self.CollectData_Ground`) :`Fertilizer` true))
          (:`then_3`
            (setmembers `/Game/Mods/StructuresPlusMod/_Structs/SP_ItemCollectorDistributeData` :`StructRef` (`self.DistributeData`) :`FertilizerToCrops` true)))))))

(fn `UserConstructionScript`
  (`parent.UserConstructionScript`))