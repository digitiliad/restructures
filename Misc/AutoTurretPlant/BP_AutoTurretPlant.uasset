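; Auto turret plant structure Blueprint that adds configurable targeting options through a turret options interface and shared SP helper functions.
; Players on the same team get a "[Turret Options]" multi-use entry, which applies a multi-tool buff.
; Stored options feed the targeting-prevention check, while the getter combines native range, AI and warning settings with stored dino level and list filters.
; HUD drawing is delegated to a shared turret helper.
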(event `self.ITurret_SetOptions`
  (params (TurretOptions :type "/Game/Mods/StructuresPlusMod/_Structs/SPTurretOptions Structure"))
  (set `self.TurretOptions` TurretOptions false))

(fn `BlueprintDrawHUD`
  (params (HUD :type "ShooterHUD Object Reference") (CenterX :type "Float (double-precision)") (CenterY :type "Float (double-precision)"))
  (`/Game/Mods/StructuresPlusMod/_Scripts/HUDFunctions.SP_Draw_HUD_-_Turret` HUD CenterX CenterY self))

(fn `BPGetMultiUseEntries`
  (params (ForPC :type "PlayerController Object Reference") (MultiUseEntries :type "Array of Actor.MultiUseEntry Structure (by ref)"))
  (returns (ReturnValue :type "Array of Actor.MultiUseEntry Structure"))
  (`|ExecutionSequence`
    (:`then_0`
      (`/Game/Mods/StructuresPlusMod/_Scripts/MultiUseMenuFunctions.SP_Clean_Up_Turret_Menu` MultiUseEntries))
    (:`then_1`
      (if (== (`Actor.TargetingTeam` ForPC) (`self.TargetingTeam`))
        (`KismetArrayLibrary.Array_Add` MultiUseEntries (make `Actor.MultiUseEntry` :`UseString` "[Turret Options]" :`UseIndex` 9001 :`Priority` -1000 :`bOverrideUseTextColor` true :`UseTextColor` (`KismetMathLibrary.Conv_LinearColorToColor` (`/Game/Mods/StructuresPlusMod/_Scripts/MultiUseMenuFunctions.SP_GetMultiUseSpecialColor`))))))
    (:`then_2`
      (return MultiUseEntries))))

(fn `BPTryMultiUse`
  (params (ForPC :type "PlayerController Object Reference") (UseIndex :type Integer))
  (returns (ReturnValue :type Boolean))
  (`|ExecutionSequence`
    (:`then_0`
      (if (== UseIndex 9001)
        (`/Game/Mods/StructuresPlusMod/_Scripts/BuffFunctions.SP_ApplyMultiToolBuff` 2 ForPC self)))
    (:`then_1`
      (return true))))

(fn `BPTurretPreventsTargeting`
  (params (PotentialTarget :type "PrimalCharacter Object Reference"))
  (returns (ReturnValue :type Boolean))
  (bind _preventtargeting (`/Game/Mods/StructuresPlusMod/_Scripts/TurretFunctions.SP_HandleTurretTargeting` PotentialTarget (`self.TurretOptions`)))
  (return _preventtargeting))

(fn `ITurret_GetOptions`
  (returns (TurretOptions :type "/Game/Mods/StructuresPlusMod/_Structs/SPTurretOptions Structure"))
  (bind ((`MinDinoLevel_14_1F75190A4BED442F21552698CA491015` _mindinolevel) (`MaxDinoLevel_16_D17219804FEC2DC4247EE0B6D1C12F38` _maxdinolevel) (`DinoList_20_49CFA23D43FDF6C83D1265B629BCA47D` _dinolist) (`IsInclusionList_29_B86BA306452A043B95545AAA17D865AD` _isinclusionlist)) (break `/Game/Mods/StructuresPlusMod/_Structs/SPTurretOptions` (`self.TurretOptions`)))
  (return (make `/Game/Mods/StructuresPlusMod/_Structs/SPTurretOptions` (`self.RangeSetting`) (`self.AISetting`) (`self.WarningSetting`) _mindinolevel _maxdinolevel _dinolist _isinclusionlist)))

(fn `UserConstructionScript`
  (`parent.UserConstructionScript`))