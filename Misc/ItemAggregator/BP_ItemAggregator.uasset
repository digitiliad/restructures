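; Structures Plus Item Aggregator: a powered container that collects items, distributes them to nearby structures and dinos, and incubates eggs.
; Server config sets slots, range and restrictions; team multi-use options open settings through a buff, returned via net exec commands.
; Settings build the ActiveScans list.
; Each repeating DoScan runs ground collection and incubation, then staggers load with one round-robin scan plus toggled vivarium or turret-ammo passes.
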(fn ConstructionScript
  (|CallParentFunction))

(fn BPServerHandleNetExecCommand
  (params (FromPC :type Player%20Controller%20Object%20Reference) (CommandName :type Name :default "None") (ExecParams :type BP%20Net%20Exec%20Params%20Structure%20%28by%20ref%29))
  (bind _objparam1 (Utilities|Struct|BreakBPNetExecParams ExecParams))
  (Utilities|FlowControl|Sequence
    (:then_0
      (Utilities|IsValid FromPC
        (:Is%20Valid
          (bind _assplus_itemcollector_comobject_c (Utilities|Casting|CastToSPlus_ItemCollector_ComObject _objparam1)
            (:then
              (switch name CommandName
                (:ItemCollector_CollectSettings
                  (Variables|Default|SetCollectData_Ground (Variables|/Game/Mods/StructuresPlusMod/_ComObjects/SPlus_ItemCollector_ComObject.SPlus_ItemCollector_ComObject_C|GetCollectData _assplus_itemcollector_comobject_c))
                  (Variables|Default|SetCollectData_Inventory (Variables|/Game/Mods/StructuresPlusMod/_ComObjects/SPlus_ItemCollector_ComObject.SPlus_ItemCollector_ComObject_C|GetInvCollectData _assplus_itemcollector_comobject_c)))
                (:ItemCollector_DistributeSettings
                  (Variables|Default|SetDistributeData (Variables|/Game/Mods/StructuresPlusMod/_ComObjects/SPlus_ItemCollector_ComObject.SPlus_ItemCollector_ComObject_C|GetDistributeData _assplus_itemcollector_comobject_c))))
              (CallFunction|GetActiveScans))
            (:CastFailed
              (bind _assplus_misc_comobject_c (Utilities|Casting|CastToSPlus_Misc_ComObject _objparam1))
              (switch name CommandName
                (:ItemCollector_CollectBlacklist
                  (Variables|Default|SetCollectionBlacklist (Variables|/Game/Mods/StructuresPlusMod/_ComObjects/SPlus_Misc_ComObject.SPlus_Misc_ComObject_C|GetObjectClasses _assplus_misc_comobject_c)))
                (:ItemCollector_CollectDestroylist
                  (Variables|Default|SetCollectionDestroylist (Variables|/Game/Mods/StructuresPlusMod/_ComObjects/SPlus_Misc_ComObject.SPlus_Misc_ComObject_C|GetObjectClasses _assplus_misc_comobject_c)))))))))
    (:then_1
      (return false))))

(fn ReceiveBeginPlay
  (bind _returnvalue (Game|GetGameMode))
  (|CallParentFunction)
  (if (not (Variables|Default|GetbIsPreviewStructure))
    (CallFunction|UpdateAnimations)
    (Networking|SwitchHasAuthority
      (:Authority
        (CallFunction|GetActiveScans)
        (Utilities|FlowControl|Sequence
          (:then_0
            (bind _value (CallFunction|SPGetConfigSetting-InventorySize _returnvalue "ItemAggregatorSlotCount" 500))
            (Variables|Default|SetInvSlotOverride _value true))
          (:then_1
            (bind _value_2 (CallFunction|SPGetConfig-Int _returnvalue "ItemAggregatorRangeInFoundations" 25 1 100))
            (Variables|Default|SetScanRadius (* _value_2 3e+02) true))
          (:then_2
            (bind _value_3 (CallFunction|SPGetConfig-Bool _returnvalue "ItemAggregatorDisableDistribution"))
            (Variables|Default|SetDisableDistribution _value_3 true))
          (:then_3
            (bind _value_4 (CallFunction|SPGetConfig-Bool _returnvalue "ItemAggregatorDisableAmmo"))
            (Variables|Default|SetDisableAmmoDistribution _value_4))
          (:then_4
            (bind _value_5 (CallFunction|SPGetConfig-Bool _returnvalue "ItemAggregatorDisableIncubation"))
            (Variables|Default|SetDisableIncubation _value_5))
          (:then_5
            (bind _value_6 (CallFunction|SPGetConfig-Float _returnvalue "ItemAggregatorIncubationMultiplier" 1.0 0.01 999999.0))
            (Variables|Default|SetIncubationMultiplier _value_6)))))))

(fn BPGetMultiUseEntries
  (params (ForPC :type Player%20Controller%20Object%20Reference) (MultiUseEntries :type Array%20of%20Multi%20Use%20Entry%20Structures))
  (bind _color (CallFunction|SPGetMultiUseSpecialColor))
  (bind _returnvalue (Math|Conversions|ToColor(LinearColor) _color))
  (bind _returnvalue_2 (|CallParentFunction ForPC MultiUseEntries))
  (Utilities|FlowControl|Sequence
    (:then_0
      (if (== (Variables|/Script/Engine.Actor|GetTargetingTeam ForPC) (Variables|Default|GetTargetingTeam))
        (Utilities|Array|Add _returnvalue_2 (Utilities|Struct|MakeMultiUseEntry "[Collection Options]" 9002 -1005 true true _returnvalue))
        (if (not (Variables|Default|GetDisableDistribution))
          (Utilities|Array|Add _returnvalue_2 (Utilities|Struct|MakeMultiUseEntry "[Distribution Options]" 9003 -1006 true true _returnvalue)))))
    (:then_1
      (return _returnvalue_2))))

(fn BPTryMultiUse
  (params (ForPC :type Player%20Controller%20Object%20Reference) (UseIndex :type Integer))
  (|CallParentFunction ForPC UseIndex)
  (Utilities|FlowControl|Sequence
    (:then_0
      (switch int UseIndex
        (:9002
          (bind _asshooterplayercontroller (Utilities|Casting|CastToShooterPlayerController ForPC))
          (bind _returnvalue (Class|PrimalBuff|StaticAddBuff "/Game/Mods/StructuresPlusMod/_Buffs/Buff_StructuresPlus_ItemAggregator.Buff_StructuresPlus_ItemAggregator_C" (Class|ShooterPlayerController|GetPlayerCharacter _asshooterplayercontroller) 0 0 false))
          (bind _asbuff_structuresplus_itemaggregator_c (Utilities|Casting|CastToBuff_StructuresPlus_ItemAggregator _returnvalue))
          (Default|InitializeUI-Collect _asbuff_structuresplus_itemaggregator_c self (Variables|Default|GetCollectData_Ground) (Variables|Default|GetCollectData_Inventory) (Variables|Default|GetCollectionBlacklist) (Variables|Default|GetCollectionDestroylist)))
        (:9003
          (bind _asshooterplayercontroller_2 (Utilities|Casting|CastToShooterPlayerController ForPC))
          (bind _returnvalue_2 (Class|PrimalBuff|StaticAddBuff "/Game/Mods/StructuresPlusMod/_Buffs/Buff_StructuresPlus_ItemAggregator.Buff_StructuresPlus_ItemAggregator_C" (Class|ShooterPlayerController|GetPlayerCharacter _asshooterplayercontroller_2) 0 0 false))
          (bind _asbuff_structuresplus_itemaggregator_c_2 (Utilities|Casting|CastToBuff_StructuresPlus_ItemAggregator _returnvalue_2))
          (Default|InitializeUI-Distribute _asbuff_structuresplus_itemaggregator_c_2 self (Variables|Default|GetDistributeData) (Variables|Default|GetDisableAmmoDistribution)))))
    (:then_1
      (return true))))

(fn BPRefreshedStructureColors
  (bind _defaultmeshmaterial (Variables|Default|GetDefaultMeshMaterial))
  (Class|KismetSystemLibrary|CanRunCosmeticEvents
    (:Yes
      (Utilities|IsValid _defaultmeshmaterial
        (:Is%20Valid
          (Rendering|Material|SetVectorParameterValue _defaultmeshmaterial "Emissive Color" (CallFunction|GetEmissiveColor) :!class /Script/Engine.MaterialInstanceDynamic))))))

(fn GetEmissiveColor
  (Utilities|FlowControl|Sequence
    (:then_0
      (if (Variables|Default|GetbContainerActivated)
        (if (Variables|Default|GetbUsingStructureColors)
          (bind _returnvalue (Class|PrimalStructure|GetStructureColor))
          (LocalVariables|SetEmissiveColor_GEC (Utilities|Struct|MakeLinearColor (.R (Utilities|Struct|BreakLinearColor _returnvalue)) (.G (Utilities|Struct|BreakLinearColor _returnvalue)) (.B (Utilities|Struct|BreakLinearColor _returnvalue)) 1e+01))
          (else
            (LocalVariables|SetEmissiveColor_GEC "(R=0.000000,G=0.321000,B=0.970000,A=1.000000)")))
        (else
          (LocalVariables|SetEmissiveColor_GEC ""))))
    (:then_1
      (return (LocalVariables|GetEmissiveColor_GEC)))))

(fn UpdateAnimations
  (bind _defaultmeshmaterial (Variables|Default|GetDefaultMeshMaterial))
  (|CallParentFunction)
  (Class|KismetSystemLibrary|CanRunCosmeticEvents
    (:Yes
      (Utilities|IsValid _defaultmeshmaterial
        (:Is%20Valid
          (Rendering|Material|SetVectorParameterValue _defaultmeshmaterial "Emissive Color" (CallFunction|GetEmissiveColor) :!class /Script/Engine.MaterialInstanceDynamic)
          (Rendering|Material|SetScalarParameterValue _defaultmeshmaterial "Emissive Power" (Math|Float|SelectFloat 2.0 9999.0 (Variables|Default|GetbContainerActivated)) :!class /Script/Engine.MaterialInstanceDynamic))))))

(fn DoScan
  (if (Variables|Default|GetbContainerActivated)
    (CallFunction|Collect-Ground)
    (CallFunction|IncubateEggs)
    (Utilities|FlowControl|Sequence
      (:then_0
        (if (Utilities|Array|IsValidIndex (Variables|Default|GetActiveScans))
          (CallFunction|DoSecondaryScan)))
      (:then_1
        (if (or (Utilities|Struct|BreakSP_ItemCollectorCollectData (Variables|Default|GetCollectData_Ground)) (Math|Boolean|ANDBoolean (not (Variables|Default|GetDisableDistribution)) (not (Variables|Default|GetDisableAmmoDistribution)) (> (Utilities|Struct|BreakSP_ItemCollectorDistributeData (Variables|Default|GetDistributeData)) 0)))
          (CallFunction|DoTertiaryScan)))
      (:then_2
        (if (Variables|Default|GetTertiaryScanToggle)
          (Class|PrimalInventoryComponent|InventoryRefresh (Variables|Default|GetMyInventoryComponent))))
      (:then_3
        (Variables|Default|SetTertiaryScanToggle (not (Variables|Default|GetTertiaryScanToggle))))
      (:then_4
        (Utilities|Time|SetTimerbyFunctionName 0 "DoScan" (CallFunction|GetScanInterval))))))

(fn DoSecondaryScan
  (Utilities|FlowControl|Sequence
    (:then_0
      (switch Utilities|FlowControl|Switch|SwitchonSP_Enum_AggregatorScanType (Utilities|Array|Get(acopy) (Variables|Default|GetActiveScans) (Variables|Default|GetSecondaryScanIndex))
        (:NewEnumerator1
          (CallFunction|Collect-BeerBarrels))
        (:NewEnumerator2
          (CallFunction|Collect-Beetles))
        (:NewEnumerator3
          (CallFunction|Collect-Charcoal))
        (:NewEnumerator4
          (CallFunction|Collect-CompostBins))
        (:NewEnumerator5
          (CallFunction|Collect-Crops))
        (:NewEnumerator6
          (CallFunction|Collect-Forges))
        (:NewEnumerator7
          (CallFunction|Collect-OilDinos))
        (:NewEnumerator8
          (CallFunction|Collect-Sheep))
        (:NewEnumerator9
          (CallFunction|Collect-Snails))
        (:NewEnumerator10
          (CallFunction|Collect-SpoiledMeat))
        (:NewEnumerator11
          (CallFunction|Collect-Turtles))
        (:NewEnumerator12
          (CallFunction|Distribute-BeerBarrels))
        (:NewEnumerator13
          (CallFunction|Distribute-Beetles))
        (:NewEnumerator14
          (CallFunction|Distribute-CompostBins))
        (:NewEnumerator15
          (CallFunction|Distribute-Crops))
        (:NewEnumerator16
          (CallFunction|Distribute-CrystalCrackers))
        (:NewEnumerator17
          (CallFunction|Distribute-DedicatedStorage))
        (:NewEnumerator18
          (CallFunction|Distribute-Forges))
        (:NewEnumerator19
          (CallFunction|Distribute-Fuel))
        (:NewEnumerator20
          (CallFunction|Distribute-Gachas))
        (:NewEnumerator21
          (CallFunction|Distribute-Troughs))))
    (:then_1
      (Variables|Default|SetSecondaryScanIndex (Math|Integer|SelectInt 0 (+ (Variables|Default|GetSecondaryScanIndex) 1) (> (+ (Variables|Default|GetSecondaryScanIndex) 1) (Utilities|Array|LastIndex (Variables|Default|GetActiveScans))))))))

(fn DoTertiaryScan
  (bind _collectdata_ground (Variables|Default|GetCollectData_Ground))
  (bind _distributedata (Variables|Default|GetDistributeData))
  (bind _vivariums (Utilities|Struct|BreakSP_ItemCollectorCollectData _collectdata_ground))
  (bind _stacksofammointurrets (Utilities|Struct|BreakSP_ItemCollectorDistributeData _distributedata))
  (bind _returnvalue (> _stacksofammointurrets 0))
  (if (and _vivariums _returnvalue)
    (if (Variables|Default|GetTertiaryScanToggle)
      (CallFunction|Distribute-Turrets)
      (else
        (CallFunction|Collect-Vivariums)))
    (elif _vivariums
      (CallFunction|Collect-Vivariums)
      (elif _returnvalue
        (CallFunction|Distribute-Turrets)))))

(fn BPContainerDeactivated
  (|CallParentFunction)
  (Networking|SwitchHasAuthority
    (:Authority
      (Utilities|Time|ClearTimerbyFunctionName 0 "DoSecondaryScan")
      (Utilities|Time|ClearTimerbyFunctionName 0 "DoTertiaryScan"))))

(fn GetActiveScans
  (bind _collectdata_ground (Variables|Default|GetCollectData_Ground))
  (bind _collectdata_inventory (Variables|Default|GetCollectData_Inventory))
  (bind _distributedata (Variables|Default|GetDistributeData))
  (bind (_wool _fertilizer _cropplots) (Utilities|Struct|BreakSP_ItemCollectorCollectData _collectdata_ground))
  (bind (_organicpolymer _snailpaste _oil _rareflowers _raremushrooms _ingots _charcoal _spoiledmeat _beer) (Utilities|Struct|BreakSP_ItemCollectorInvCollectData _collectdata_inventory))
  (bind (_pooptobins _pooptobeetles _gachatocracker _pelletstogacha _fertilizertocrops _uploadtodedicatedstorage _stacksoffoodintroughs _thatchtobins _thatchtobarrels _berriestobarrels _metaltoforges _stacksoffuel) (Utilities|Struct|BreakSP_ItemCollectorDistributeData _distributedata))
  (Utilities|Array|Clear (Variables|Default|GetActiveScans))
  (Variables|Default|SetSecondaryScanIndex 0)
  (Utilities|FlowControl|Sequence
    (:then_0
      (if _gachatocracker
        (CallFunction|AddScanType "NewEnumerator16")))
    (:then_1
      (if (> _pelletstogacha 0)
        (CallFunction|AddScanType "NewEnumerator20")))
    (:then_2
      (if _fertilizer
        (CallFunction|AddScanType "NewEnumerator4")))
    (:then_3
      (if (or _pooptobins _thatchtobins)
        (CallFunction|AddScanType "NewEnumerator14")))
    (:then_4
      (if _fertilizer
        (CallFunction|AddScanType "NewEnumerator2")))
    (:then_5
      (if _pooptobeetles
        (CallFunction|AddScanType "NewEnumerator13")))
    (:then_6
      (if _cropplots
        (CallFunction|AddScanType "NewEnumerator5")))
    (:then_7
      (if _fertilizertocrops
        (CallFunction|AddScanType "NewEnumerator15")))
    (:then_8
      (if (or _thatchtobarrels _berriestobarrels)
        (CallFunction|AddScanType "NewEnumerator12")))
    (:then_9
      (if _spoiledmeat
        (CallFunction|AddScanType "NewEnumerator10")))
    (:then_10
      (if (> _stacksoffoodintroughs 0)
        (CallFunction|AddScanType "NewEnumerator21")))
    (:then_11
      (if _wool
        (CallFunction|AddScanType "NewEnumerator8")))
    (:then_12
      (if (or _organicpolymer _snailpaste)
        (CallFunction|AddScanType "NewEnumerator9")))
    (:then_13
      (if (or _rareflowers _raremushrooms)
        (CallFunction|AddScanType "NewEnumerator11")))
    (:then_14
      (if _oil
        (CallFunction|AddScanType "NewEnumerator7")))
    (:then_15
      (if _ingots
        (CallFunction|AddScanType "NewEnumerator6")))
    (:then_16
      (if _charcoal
        (CallFunction|AddScanType "NewEnumerator3")))
    (:then_17
      (if (> _stacksoffuel 0)
        (CallFunction|AddScanType "NewEnumerator19")))
    (:then_18
      (if _metaltoforges
        (CallFunction|AddScanType "NewEnumerator18")))
    (:then_19
      (if _beer
        (CallFunction|AddScanType "NewEnumerator1")))
    (:then_20
      (if _uploadtodedicatedstorage
        (CallFunction|AddScanType "NewEnumerator17")))))

(fn BPContainerActivated
  (|CallParentFunction)
  (Networking|SwitchHasAuthority
    (:Authority
      (CallFunction|GetActiveScans))))

(fn AddScanType
  (params (ScanType :type SP_Enum_AggregatorScanType%20Enum :default "NewEnumerator0"))
  (Utilities|Array|Add (Variables|Default|GetActiveScans) ScanType))