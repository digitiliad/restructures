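; Industrial cooker structure, a powered-style crafting station with team-aware lock access and an auto-crafting toggle in its multi-use menu.
; On authority BeginPlay it reads slot count, crafting speed, storm disabling and noise settings from game mode config through SP helpers.
; RepNotifies apply slot count, auto-craft checking and emitter muting to components.
; The placement check overrides one specific rejection code (-9).
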(fn `BPCanBeActivatedByPlayer`
  (params (PC :type "ShooterPlayerController Object Reference"))
  (returns (ReturnValue :type Boolean))
  (return (or (== (`Actor.TargetingTeam` PC) (`self.TargetingTeam`)) (not (`self.bIsLocked`)))))

(fn `BPGetMultiUseEntries`
  (params (ForPC :type "PlayerController Object Reference") (MultiUseEntries :type "Array of Actor.MultiUseEntry Structure (by ref)"))
  (returns (ReturnValue :type "Array of Actor.MultiUseEntry Structure"))
  (bind _entriesout (`/Game/Mods/StructuresPlusMod/_Scripts/MultiUseMenuFunctions.SP_Update_Multi_Use_Menu` ForPC MultiUseEntries self))
  (`|ExecutionSequence`
    (:`then_0`
      (bind _returnvalue (`self.AllowStructureAccess` ForPC))
      (if _returnvalue
        (`KismetArrayLibrary.Array_Add` _entriesout (make `Actor.MultiUseEntry` :`UseString` (`KismetMathLibrary.SelectString` "Enable Auto Crafting" "Disable Auto Crafting" (`self.DisableAutoCrafting`)) :`UseIndex` 9002 :`Priority` -1020 :`bHideFromUI` true :`bDisplayOnInventoryUITertiary` true))))
    (:`then_1`
      (return _entriesout))))

(fn `BPIsAllowedToBuild`
  (params (OutPlacementData :type "PrimalStructure.PlacementData Structure (by ref)") (CurrentAllowedReason :type Integer))
  (returns (ReturnValue :type Integer))
  (return (`KismetMathLibrary.SelectInt` 1 CurrentAllowedReason (== CurrentAllowedReason -9))))

(fn `BPTryMultiUse`
  (params (ForPC :type "PlayerController Object Reference") (UseIndex :type Integer))
  (returns (ReturnValue :type Boolean))
  (`|ExecutionSequence`
    (:`then_0`
      (switch `int` UseIndex
        (:`Default`
          (switch `int` UseIndex
            (:`9002`
              (set `self.DisableAutoCrafting` (not (`self.DisableAutoCrafting`)) true))))
        (:`601`
          (set `self.IsUnlocked` (not (`self.bIsLocked`))))))
    (:`then_1`
      (return true))))

(fn `OnRep_DisableAutoCrafting`
  (set `PrimalInventoryComponent.bCheckForAutoCraftBlueprints` (not (`self.DisableAutoCrafting`)) (`self.MyInventoryComponent`)))

(fn `OnRep_DisableSound`
  (if (`KismetSystemLibrary.IsDedicatedServer`)
    _
    (elif (`self.DisableSound`)
      (bind _asprimalemitterspawnable (cast `PrimalEmitterSpawnable` (`ChildActorComponent.ChildActor` (`self.ActivatedEmitter`))))
      (`AudioComponent.SetVolumeMultiplier` (`PrimalEmitterSpawnable.SoundToPlay` _asprimalemitterspawnable) 0.0))))

(fn `OnRep_InventorySlots`
  (set `PrimalInventoryComponent.MaxInventoryItems` (`self.InventorySlots`) (`self.MyInventoryComponent`)))

(fn `ReceiveBeginPlay`
  (bind _returnvalue (`GameplayStatics.GetGameMode`))
  (`parent.ReceiveBeginPlay`)
  (if (not (`self.bIsPreviewStructure`))
    (`/Engine/EditorBlueprintResources/ActorMacros.Switch Has Authority`
      (:`Authority`
        (`|ExecutionSequence`
          (:`then_0`
            (bind _value (`/Game/Mods/StructuresPlusMod/_Scripts/ConfigFunctions.SP_GetConfigSetting_-_InventorySize` _returnvalue "IndustrialCookerSlotCount" 100))
            (set `self.InventorySlots` _value true))
          (:`then_1`
            (bind _value_2 (`/Game/Mods/StructuresPlusMod/_Scripts/ConfigFunctions.SP_GetConfigSetting_-_StormDisableElectronics` _returnvalue))
            (set `self.bDisableStructureOnElectricStorm` _value_2))
          (:`then_2`
            (bind _value_3 (`/Game/Mods/StructuresPlusMod/_Scripts/ConfigFunctions.SP_GetConfig_-_Float` _returnvalue "IndustrialCookingPotCraftingSpeed" 12.0 1.0 100.0))
            (set `PrimalInventoryComponent.CraftingItemSpeed` _value_3 (`self.MyInventoryComponent`)))
          (:`then_3`
            (bind _disablesound (`/Game/Mods/StructuresPlusMod/_Scripts/ConfigFunctions.SP_GetConfigSetting_-_Noise` _returnvalue))
            (set `self.DisableSound` _disablesound true))
          (:`then_4`
            (set `self.bIsLocked` (not (`self.IsUnlocked`)) true))
          (:`then_5`
            (`/Engine/EditorBlueprintResources/ActorMacros.SwitchNetAuthority`
              (:`PlayerServer`
                (`self.OnRep_DisableAutoCrafting`)))))))))

(fn `UserConstructionScript`
  (`parent.UserConstructionScript`))