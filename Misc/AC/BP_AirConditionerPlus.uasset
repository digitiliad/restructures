(event `HandleBeginPlayEvent`
  (bind _linkedstructures (`self.LinkedStructures`))
  (`KismetSystemLibrary.Delay` 1.0)
  (for _array_element _linkedstructures
    (cast `/Misc/AC/BP_AirConditionerPlus` _array_element)
    (`KismetArrayLibrary.Array_Clear` (`PrimalStructure.LinkedStructures` _array_element)))
  (`KismetArrayLibrary.Array_Clear` _linkedstructures))

(event `Key|G`
  (bind _returnvalue (not (`self.SnapsDisabled`)))
  (:`Pressed`
    (bind _returnvalue_2 (`self.GetOwnerController`))
    (bind _success (`/Game/Mods/StructuresPlusMod/_Scripts/GlobalBuffFunctions.SP_ToggleGlobalBuffDisabledSnaps` _returnvalue_2 (`|MakeArray`) (`|MakeArray` 1) _returnvalue))
    (if _success
      (set `self.SnapsDisabled` _returnvalue))))

(fn `BPGetMultiUseEntries`
  (params (ForPC :type "PlayerController Object Reference") (MultiUseEntries :type "Array of Actor.MultiUseEntry Structure (by ref)"))
  (returns (ReturnValue :type "Array of Actor.MultiUseEntry Structure"))
  (bind _entriesout (`/Game/Mods/StructuresPlusMod/_Scripts/MultiUseMenuFunctions.SP_Update_Multi_Use_Menu` ForPC MultiUseEntries self))
  (return _entriesout))

(fn `BPIsAllowedToBuild`
  (params (OutPlacementData :type "PrimalStructure.PlacementData Structure (by ref)") (CurrentAllowedReason :type Integer))
  (returns (ReturnValue :type Integer))
  (set `self.IsSnappedToWindowWall` (`KismetMathLibrary.ClassIsChildOf` (`GameplayStatics.GetObjectClass` (`.ParentStructure` (break `PrimalStructure.PlacementData` OutPlacementData))) "/Game/PrimalEarth/Structures/BuildingBases/WindowWall_Base_SM.WindowWall_Base_SM_C") false)
  (return (`KismetMathLibrary.SelectInt` 1 CurrentAllowedReason (== CurrentAllowedReason -9))))

(fn `BPSetPlayerConstructor`
  (params (PC :type "PlayerController Object Reference"))
  (bind _asbuff_structuresplus_globalbuff_c (cast `/Game/Mods/StructuresPlusMod/_Buffs/Buff_StructuresPlus_GlobalBuff` (`/Game/Mods/StructuresPlusMod/_Scripts/GlobalBuffFunctions.SP_GetGlobalBuff` PC)))
  (set `self.SnapsDisabled` (> (`KismetArrayLibrary.Array_Length` (`/Game/Mods/StructuresPlusMod/_Buffs/Buff_StructuresPlus_GlobalBuff.DisabledSnapsFrom` _asbuff_structuresplus_globalbuff_c)) 0))
  (`/Game/Mods/StructuresPlusMod/_Scripts/GlobalBuffFunctions.SP_ClearGlobalBuffDisabledSnaps` PC))

(fn `IsValidSnapPointFrom`
  (params (ParentStructure :type "PrimalStructure Object Reference") (MySnapPointFromIndex :type Integer))
  (returns (ReturnValue :type Boolean))
  (return (not (`self.SnapsDisabled`))))

(fn `IsValidSnapPointTo`
  (params (ChildStructure :type "PrimalStructure Object Reference") (MySnapPointToIndex :type Integer))
  (returns (ReturnValue :type Boolean))
  (return (not (`self.IsSnappedToWindowWall`))))

(fn `ReceiveBeginPlay`
  (`parent.ReceiveBeginPlay`)
  (if (`self.bIsPreviewStructure`)
    (bind _returnvalue (`self.GetOwnerController`))
    (`self.EnableInput` _returnvalue)
    (`/Game/Mods/StructuresPlusMod/_Scripts/GlobalBuffFunctions.SP_ClearGlobalBuffDisabledSnaps` _returnvalue)
    (else
      (`/Engine/EditorBlueprintResources/ActorMacros.Switch Has Authority`
        (:`Authority`
          (`self.HandleBeginPlayEvent`))))))

(fn `UserConstructionScript`)