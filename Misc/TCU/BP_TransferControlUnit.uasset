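; S+ Transfer Control Unit (TCU): a placeable structure that bulk-transfers items within a configured range using the active preset.
; Multi-use menus select presets or open the OmniTool buff's editor, which syncs through net exec commands and com objects.
; Activation or PIN entry triggers cooldown-gated transfers, with an emissive material showing active state until server-side reset.
; Per-team custom actor lists enforce the configurable tribe placement limit.
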(event Custom|HandleBeginPlayEvent
  (Utilities|FlowControl|Delay 1.0)
  (CallFunction|SPAddtoCustomActorList self (Utilities|String|BuildString(Integer) "SPlusTCUs_" "" (Variables|Default|GetTargetingTeam))))

(event EventBPContainerActivated
  (bind _activemat (Variables|Default|GetActiveMat))
  (Utilities|FlowControl|Sequence
    (:then_0
      (Utilities|IsValid _activemat
        (:Is%20Valid
          (Rendering|Material|SetVectorParameterValue _activemat "Emissive - Color and Intensity" "(R=0.000000,G=1.000000,B=0.165230,A=2.000000)" :!class /Script/Engine.MaterialInstanceDynamic))))
    (:then_1
      (Class|KismetSystemLibrary|IsRunningonServer
        (:Yes
          (Utilities|FlowControl|Delay (Variables|Default|GetPullCooldown))
          (Class|PrimalStructure|SetContainerActive false))))))

(event EventBPContainerDeactivated
  (bind _activemat (Variables|Default|GetActiveMat))
  (Utilities|IsValid _activemat
    (:Is%20Valid
      (Rendering|Material|SetVectorParameterValue _activemat "Emissive - Color and Intensity" "(R=0.000000,G=0.000000,B=0.000000,A=1.000000)" :!class /Script/Engine.MaterialInstanceDynamic))))

(fn ConstructionScript
  (|CallParentFunction)
  (if (and (not (Variables|Default|GetbIsPreviewStructure)) (not (Networking|IsDedicatedServer)))
    (bind _returnvalue (Rendering|Material|CreateDynamicMaterialInstance "/Game/Genesis/Dinos/HLNA/HLN_A_Colorized_MIC.HLN_A_Colorized_MIC" :!class /Script/Engine.KismetMaterialLibrary))
    (Variables|Default|SetActiveMat _returnvalue)
    (Rendering|Material|SetMaterial (Variables|Default|GetStaticMesh1) 0 _returnvalue)
    (Rendering|Material|SetVectorParameterValue :self _returnvalue :ParameterName "Emissive - Color and Intensity" :!class /Script/Engine.MaterialInstanceDynamic)))

(fn BPGetMultiUseEntries
  (params (ForPC :type Player%20Controller%20Object%20Reference) (MultiUseEntries :type Array%20of%20Multi%20Use%20Entry%20Structures))
  (bind _color (CallFunction|SPGetMultiUseSpecialColor))
  (bind _self self)
  (bind _returnvalue (Math|Conversions|ToColor(LinearColor) _color))
  (bind _entriesout (CallFunction|SPUpdateMultiUseMenu ForPC MultiUseEntries _self false false false false))
  (Utilities|FlowControl|Sequence
    (:then_0
      (bind _accesslevel (CallFunction|SPGetAccessLevel ForPC _self))
      (if (>= _accesslevel 2)
        (Utilities|Array|Add _entriesout (Utilities|Struct|MakeMultiUseEntry "[Edit Transfers]" 9000 -1000 true _returnvalue))
        (Utilities|Array|Add _entriesout (Utilities|Struct|MakeMultiUseEntry "[Set Active Transfer]" 9001 -1000 true true true _returnvalue))
        (for (_array_element _array_index) (Variables|Default|GetPresetNames)
          (Utilities|Array|Add _entriesout (Utilities|Struct|MakeMultiUseEntry _array_element (+ _array_index 9002) _array_index (== _array_index (Variables|Default|GetActiveTransferIndex)) 9001 _returnvalue)))))
    (:then_1
      (return _entriesout))))

(fn ReceiveBeginPlay
  (|CallParentFunction)
  (if (not (Variables|Default|GetbIsPreviewStructure))
    (Networking|SwitchHasAuthority
      (:Authority
        (Utilities|FlowControl|Sequence
          (:then_0
            (bind (_disablepulling _pullrange _cooldown) (CallFunction|SPGetConfigSetting-Pull (Game|GetGameMode)))
            (Variables|Default|SetPullRange _pullrange)
            (Variables|Default|SetPullCooldown _cooldown false)))))))

(fn BPTryMultiUse
  (params (ForPC :type Player%20Controller%20Object%20Reference) (UseIndex :type Integer))
  (Utilities|FlowControl|Sequence
    (:then_0
      (switch int UseIndex
        (:Default
          (if (== UseIndex 600)
            (CallFunction|PerformTransfer ForPC)))
        (:9000
          (bind _asshooterplayercontroller (Utilities|Casting|CastToShooterPlayerController ForPC))
          (bind _returnvalue (Class|PrimalBuff|StaticAddBuff "/Game/Mods/StructuresPlusMod/_Buffs/Buff_StructuresPlus_OmniTool.Buff_StructuresPlus_OmniTool_C" (Class|ShooterPlayerController|GetPlayerCharacter _asshooterplayercontroller) 0 0 false))
          (bind _asbuff_structuresplus_omnitool_c (Utilities|Casting|CastToBuff_StructuresPlus_OmniTool _returnvalue))
          (Default|Transfer-InitializeUIfromStructure _asbuff_structuresplus_omnitool_c self (Variables|Default|GetPresets) (Variables|Default|GetPresetNames)))
        (:9002
          (Variables|Default|SetActiveTransferIndex 0 true))
        (:9003
          (Variables|Default|SetActiveTransferIndex 1 true))
        (:9004
          (Variables|Default|SetActiveTransferIndex 2 true))
        (:9005
          (Variables|Default|SetActiveTransferIndex 3 true))
        (:9006
          (Variables|Default|SetActiveTransferIndex 4 true))))
    (:then_1
      (return true))))

(fn BPServerHandleNetExecCommand
  (params (FromPC :type Player%20Controller%20Object%20Reference) (CommandName :type Name :default "None") (ExecParams :type BP%20Net%20Exec%20Params%20Structure%20%28by%20ref%29))
  (bind (_intparam1 _objparam1 _stringparam1) (Utilities|Struct|BreakBPNetExecParams ExecParams))
  (bind _presets (Variables|Default|GetPresets))
  (Utilities|FlowControl|Sequence
    (:then_0
      (switch name CommandName
        (:SetPreset
          (bind _assplus_omnitool_comobject_c (Utilities|Casting|CastToSPlus_Omnitool_ComObject _objparam1))
          (if (Utilities|Array|IsValidIndex (Variables|/Game/Mods/StructuresPlusMod/_ComObjects/SPlus_Omnitool_ComObject.SPlus_Omnitool_ComObject_C|GetTransferData _assplus_omnitool_comobject_c))
            (Utilities|Array|SetArrayElem (Variables|Default|GetPresets) _intparam1 (Utilities|Array|Get(acopy) (Variables|/Game/Mods/StructuresPlusMod/_ComObjects/SPlus_Omnitool_ComObject.SPlus_Omnitool_ComObject_C|GetTransferData _assplus_omnitool_comobject_c)))))
        (:SetPresetName
          (Utilities|Array|SetArrayElem (Variables|Default|GetPresetNames) _intparam1 _stringparam1)
          (Class|Actor|MulticastProperty "PresetNames"))
        (:ApplyPresets
          (bind _assplus_omnitool_comobject_c_2 (Utilities|Casting|CastToSPlus_Omnitool_ComObject _objparam1))
          (Utilities|Array|Clear _presets)
          (Utilities|Array|AppendArray _presets (Variables|/Game/Mods/StructuresPlusMod/_ComObjects/SPlus_Omnitool_ComObject.SPlus_Omnitool_ComObject_C|GetTransferData _assplus_omnitool_comobject_c_2)))
        (:GetTransferPresetsFromStructure
          (bind _asprimalbuff (Utilities|Casting|CastToPrimalBuff _objparam1))
          (bind _returnvalue (Class|VictoryCore|ConstructObjectAutoNameBP "/Game/Mods/StructuresPlusMod/_ComObjects/SPlus_Omnitool_ComObject.SPlus_Omnitool_ComObject_C" _asprimalbuff))
          (bind _assplus_omnitool_comobject_c_3 (Utilities|Casting|CastToSPlus_Omnitool_ComObject _returnvalue))
          (Utilities|Array|AppendArray (Variables|/Game/Mods/StructuresPlusMod/_ComObjects/SPlus_Omnitool_ComObject.SPlus_Omnitool_ComObject_C|GetTransferData _assplus_omnitool_comobject_c_3) (Variables|Default|GetPresets))
          (CallFunction|BPServerHandleNetExecCommand _asprimalbuff FromPC "GetTransferPresetsFromStructure" (Utilities|Struct|MakeBPNetExecParams _assplus_omnitool_comobject_c_3))
          (for (_array_element _array_index) (Variables|Default|GetPresetNames)
            (CallFunction|BPServerHandleNetExecCommand _asprimalbuff FromPC "Transfer_SavePresetName" (Utilities|Struct|MakeBPNetExecParams _array_index _array_element))))))
    (:then_1
      (return true))))

(fn BPCanbeActivatedbyPlayer
  (params (PC :type Shooter%20Player%20Controller%20Object%20Reference))
  (return (and (>= (Class|VictoryCore|GetNetworkTimeinSeconds) (+ (Variables|Default|GetLastPullTime) (Variables|Default|GetPullCooldown))) (not (Variables|Default|GetbContainerActivated)))))

(fn PerformTransfer
  (params (PC :type Player%20Controller%20Object%20Reference))
  (bind _presets (Variables|Default|GetPresets))
  (bind _activetransferindex (Variables|Default|GetActiveTransferIndex))
  (if (>= (Class|VictoryCore|GetNetworkTimeinSeconds) (+ (Variables|Default|GetLastPullTime) (Variables|Default|GetPullCooldown)))
    (if (Utilities|Array|IsValidIndex _presets _activetransferindex)
      (bind _log (CallFunction|SPDoBulkTransfer PC (Utilities|Array|Get(acopy) _presets _activetransferindex) (Transformation|GetActorLocation) (Variables|Default|GetPullRange)))
      (Utilities|FlowControl|Sequence
        (:then_0
          (if (Utilities|Array|IsValidIndex _log (Utilities|Array|LastIndex _log))
            (Class|StructuresPlus|SPMessageClient PC (Utilities|Array|Get(acopy) _log (Utilities|Array|LastIndex _log)) "Default")))
        (:then_1
          (Variables|Default|SetLastPullTime (Class|VictoryCore|GetNetworkTimeinSeconds) true))))))

(fn BPClientDoMultiUse
  (params (ForPC :type Player%20Controller%20Object%20Reference) (ClientUseIndex :type Integer))
  (bind _asshooterplayercontroller (Utilities|Casting|CastToShooterPlayerController ForPC))
  (switch int ClientUseIndex
    (:9001
      (Class|ShooterPlayerController|SetMultiUseWheelCategory _asshooterplayercontroller ClientUseIndex))))

(fn BPConsumeUsePinCode
  (params (FromKeypadActor :type Actor%20Object%20Reference) (ForPC :type Player%20Controller%20Object%20Reference) (appledPinCode :type Integer) (bIsActivating :type Boolean))
  (Utilities|FlowControl|Sequence
    (:then_0
      (if (and bIsActivating (Class|PrimalStructureItemContainer|VerifyPinCode appledPinCode))
        (CallFunction|PerformTransfer ForPC)))
    (:then_1
      (return false))))

(fn BPIsAllowedtoBuildEx
  (params (OutPlacementData :type Placement%20Data%20Structure%20%28by%20ref%29) (CurrentAllowedReason :type Integer) (PC :type Player%20Controller%20Object%20Reference) (bFinalPlacement :type Boolean) (bChoosingRotation :type Boolean))
  (LocalVariables|SetBuildReasonEx CurrentAllowedReason)
  (Utilities|FlowControl|Sequence
    (:then_0
      (if (and (> (LocalVariables|GetBuildReasonEx) 0) bFinalPlacement)
        (Class|KismetSystemLibrary|IsRunningonServer
          (:Yes
            (bind _value (CallFunction|SPGetConfig-Int (Game|GetGameMode) "TribeTCULimit" 0 0 999999))
            (if (> _value 0)
              (bind _count (CallFunction|SPCountValidActorsinActorList self (Utilities|String|BuildString(Integer) "SPlusTCUs_" "" (Variables|Default|GetTargetingTeam))))
              (if (>= _count _value)
                (LocalVariables|SetBuildReasonEx -699)
                (Class|StructuresPlus|SPMessageClient PC (Utilities|String|BuildString(Integer) "Your tribe has reached its TCU limit." " (" _value ")") "Error")
                (else
                  (Class|StructuresPlus|SPMessageClient PC (Utilities|String|BuildString(Integer) "Your tribe can place " "" (- _value (+ _count 1)) (Utilities|String|SelectString " more TCU." " more TCUs." (== (- _value (+ _count 1)) 1))) "Default"))))))))
    (:then_1
      (return (LocalVariables|GetBuildReasonEx)))))

(fn ReceiveDestroyed
  (Networking|SwitchHasAuthority
    (:Authority
      (if (not (Variables|Default|GetbIsPreviewStructure))
        (CallFunction|SPRemovefromCustomActorList self (Utilities|String|BuildString(Integer) "SPlusTCUs_" "" (Variables|Default|GetTargetingTeam)))))))

(fn BPonStructurePickup
  (params (PlayerController :type Player%20Controller%20Object%20Reference) (ItemType :type Primal%20Item%20Class%20Reference) (NewlyPickedUpItem :type Primal%20Item%20Object%20Reference) (bIsQuickPickup :type Boolean))
  (Networking|SwitchHasAuthority
    (:Authority
      (CallFunction|SPRemovefromCustomActorList self (Utilities|String|BuildString(Integer) "SPlusTCUs_" "" (Variables|Default|GetTargetingTeam))))))