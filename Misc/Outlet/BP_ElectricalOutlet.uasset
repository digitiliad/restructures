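; Electrical outlet structure with same-team multi-use options to hide its mesh, toggle sparks and hide nearby wires.
; RepNotify flags drive mesh visibility and the child spark emitter's template, while a game-mode setting can disable hiding and decayed outlets unhide on BeginPlay.
; Wire hiding is one-way: a multicast, or delayed RepNotify, sphere-overlaps nearby item containers and hides their cable particles.
; Placement checks override one specific build-rejection code.
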(event Custom|MulticastWireHide
  (Utilities|SwitchNetAuthority
    (:PlayerServer
      _)
    (:Client
      _))
  (CallFunction|HideConnectingWires))

(event Custom|ToggleConnectorsVisibilityEvent
  (Utilities|FlowControl|Delay 2.5)
  (CallFunction|HideConnectingWires))

(fn ConstructionScript)

(fn BPIsAllowedtoBuild
  (params (OutPlacementData :type Placement%20Data%20Structure%20%28by%20ref%29) (CurrentAllowedReason :type Integer))
  (return (Math|Integer|SelectInt 1 CurrentAllowedReason (== CurrentAllowedReason -9))))

(fn BPGetMultiUseEntries
  (params (ForPC :type Player%20Controller%20Object%20Reference) (MultiUseEntries :type Array%20of%20Multi%20Use%20Entry%20Structures))
  (bind _entriesout (CallFunction|SPUpdateMultiUseMenu ForPC MultiUseEntries self false false false false))
  (Utilities|FlowControl|Sequence
    (:then_0
      (if (== (Variables|/Script/Engine.Actor|GetTargetingTeam ForPC) (Variables|Default|GetTargetingTeam))
        (if (Variables|Default|GetDisableHide)
          _
          (else
            (Utilities|Array|Add _entriesout (Utilities|Struct|MakeMultiUseEntry (Utilities|String|SelectString "Show" "Hide" (Variables|Default|GetIsHidden)) 9001 -1001 false))))
        (Utilities|Array|Add _entriesout (Utilities|Struct|MakeMultiUseEntry (Utilities|String|SelectString "Enable Sparks" "Disable Sparks" (Variables|Default|GetAreSparksHidden)) 9002 -1002 false))
        (Utilities|Array|Add _entriesout (Utilities|Struct|MakeMultiUseEntry (Utilities|String|SelectString "Force Hide Nearby Wires" "Hide Nearby Wires" (Variables|Default|GetAreWiresHidden)) 9003 -1003 false))))
    (:then_1
      (return _entriesout))))

(fn BPTryMultiUse
  (params (ForPC :type Player%20Controller%20Object%20Reference) (UseIndex :type Integer))
  (Utilities|FlowControl|Sequence
    (:then_0
      (switch int UseIndex
        (:9001
          (Variables|Default|SetIsHidden (not (Variables|Default|GetIsHidden)) true))
        (:9002
          (Variables|Default|SetAreSparksHidden (not (Variables|Default|GetAreSparksHidden)) true))
        (:9003
          (CallFunction|MulticastWireHide)
          (Variables|Default|SetAreWiresHidden true true))))
    (:then_1
      (return false))))

(fn HideConnectingWires
  (bind (_outactors _returnvalue) (Class|KismetSystemLibrary|SphereOverlapActorsSimple (Transformation|GetActorLocation) 1e+03 "ObjectTypeQuery9" "/Script/ShooterGame.PrimalStructureItemContainer" (Utilities|Array|MakeArray self)))
  (if _returnvalue
    (for _array_element _outactors
      (bind _asprimalstructureitemcontainer (Utilities|Casting|CastToPrimalStructureItemContainer _array_element))
      (Development|SetHiddeninGame (Variables|/Script/ShooterGame.PrimalStructureItemContainer|GetJunctionLinkCableParticle _asprimalstructureitemcontainer) true true)
      (Rendering|SetVisibility (Variables|/Script/ShooterGame.PrimalStructureItemContainer|GetJunctionLinkCableParticle _asprimalstructureitemcontainer) false true))))

(fn OnRepAreWiresHidden
  (Utilities|SwitchNetAuthority
    (:PlayerServer
      _)
    (:Client
      _))
  (CallFunction|ToggleConnectorsVisibilityEvent))

(fn ReceiveBeginPlay
  (|CallParentFunction)
  (if (not (Variables|Default|GetbIsPreviewStructure))
    (Networking|SwitchHasAuthority
      (:Authority
        (Utilities|FlowControl|Sequence
          (:then_0
            (bind _disablehide (CallFunction|SPGetConfigSetting-Hide (Game|GetGameMode)))
            (Variables|Default|SetDisableHide _disablehide true))
          (:then_1
            (Utilities|SwitchNetAuthority
              (:PlayerServer
                (CallFunction|OnRepIsHidden)
                (CallFunction|OnRepAreSparksHidden)
                (CallFunction|OnRepAreWiresHidden))))
          (:then_2
            (if (and (Variables|Default|GetIsHidden) (CallFunction|SPHasStructureDecayed self))
              (Variables|Default|SetIsHidden false true))))))))

(fn OnRepIsHidden
  (Rendering|SetVisibility (Variables|Default|GetMyStaticMesh) (or (Variables|Default|GetDisableHide) (not (Variables|Default|GetIsHidden))) false))

(fn OnRepAreSparksHidden
  (bind _asjunctionsparksemitter_c (Utilities|Casting|CastToJunctionSparksEmitter (Variables|/Script/Engine.ChildActorComponent|GetChildActor (Variables|Default|GetActivatedEmitter))))
  (if (Variables|Default|GetAreSparksHidden)
    (Effects|Components|ParticleSystem|SetTemplate _asjunctionsparksemitter_c 0)
    (else
      (Effects|Components|ParticleSystem|SetTemplate _asjunctionsparksemitter_c "/Game/FirePack/Particles/P_Sparks.P_Sparks")
      (if (Variables|Default|GetbContainerActivated)
        (Components|Activation|Activate _asjunctionsparksemitter_c false)))))