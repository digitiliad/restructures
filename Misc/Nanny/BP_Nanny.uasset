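; ARK Nanny structure that feeds and imprints nearby same-tribe or allied babies that have an imprinter.
; While activated, a timed octree scan raises imprint toward baby age up to a cap, using the previous scan's list.
; It feeds hungry young babies from its inventory using cached per-species food lists sorted by ascending affinity, unstasising them first.
; Server config sets limits and timing, while wheel menus set transfer amount and toggle imprinting.
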(event Custom|ForceUpdateImprintingEvent
  (params (Dino :type Primal%20Dino%20Character%20Object%20Reference) (ImprintValue :type Float%20%28single-precision%29))
  (Utilities|SwitchNetAuthority
    (:Client
      (bind _returnvalue (Class|PrimalCharacter|GetCharacterStatusComponent Dino))
      (Variables|/Script/ShooterGame.PrimalCharacterStatusComponent|SetDinoImprintingQuality _returnvalue ImprintValue false))))

(fn ConstructionScript
  (|CallParentFunction))

(fn GetDinos
  (bind _targetingteam (Variables|Default|GetTargetingTeam))
  (bind _asshootergamemode (Utilities|Casting|CastToShooterGameMode (Game|GetGameMode)))
  (bind _returnvalue (Class|VictoryCore|ServerOctreeOverlapActorsClass (Class|Actor|GetWorld) (Transformation|GetActorLocation) (Variables|Default|GetScanRadius) "DINOPAWNS" "/Script/ShooterGame.PrimalDinoCharacter" true))
  (for _array_element _returnvalue
    (bind _returnvalue_2 (Class|ShooterGameMode|AreTribesAllied _asshootergamemode (Variables|/Script/Engine.Actor|GetTargetingTeam _array_element) _targetingteam))
    (if (or _returnvalue_2 (== (Variables|/Script/Engine.Actor|GetTargetingTeam _array_element) _targetingteam))
      (bind _asprimaldinocharacter (Utilities|Casting|CastToPrimalDinoCharacter _array_element))
      (if (and (Utilities|Enum|NotEqual(Enum) (Variables|/Script/ShooterGame.PrimalDinoCharacter|GetImprinterName _asprimaldinocharacter) "") (not (Variables|/Script/ShooterGame.PrimalCharacter|GetbIsDead _asprimaldinocharacter)))
        (Utilities|FlowControl|Sequence
          (:then_0
            (if (< (Variables|/Script/ShooterGame.PrimalDinoCharacter|GetBabyAge _asprimaldinocharacter) 1.0)
              (Utilities|Array|Add (LocalVariables|GetDinosToImprint) _asprimaldinocharacter)
              (if (Variables|/Script/ShooterGame.PrimalDinoCharacter|GetbEnableTamedWandering _asprimaldinocharacter)
                (Variables|/Script/ShooterGame.PrimalDinoCharacter|SetbEnableTamedWandering _asprimaldinocharacter false false)
                (Class|Actor|MulticastProperty _asprimaldinocharacter "bEnableTamedWandering"))))
          (:then_1
            (if (<= (Variables|/Script/ShooterGame.PrimalDinoCharacter|GetBabyAge _asprimaldinocharacter) 0.15)
              (Utilities|Array|Add (LocalVariables|GetDinosToFeed) _asprimaldinocharacter)))))))
  (return (LocalVariables|GetDinosToFeed) (LocalVariables|GetDinosToImprint)))

(fn HandleImprinting
  (params (Dinos :type Array%20of%20Primal%20Dino%20Character%20Object%20References))
  (bind _maximprint (Variables|Imprinting|GetMaxImprint))
  (for _array_element Dinos
    (Utilities|IsValid _array_element
      (:Is%20Valid
        (Utilities|FlowControl|Sequence
          (:then_0
            (if (Variables|/Script/Engine.Actor|GetbStasised _array_element)
              (Class|Actor|Unstasis _array_element)))
          (:then_1
            (bind _returnvalue (Class|PrimalCharacter|GetCharacterStatusComponent _array_element))
            (if (and (> _maximprint (Variables|/Script/ShooterGame.PrimalCharacterStatusComponent|GetDinoImprintingQuality _returnvalue)) (< (Variables|/Script/ShooterGame.PrimalCharacterStatusComponent|GetDinoImprintingQuality _returnvalue) (Variables|/Script/ShooterGame.PrimalDinoCharacter|GetBabyAge _array_element)))
              (Variables|/Script/ShooterGame.PrimalCharacterStatusComponent|SetDinoImprintingQuality _returnvalue (Math|Float|Min(Float) _maximprint (Variables|/Script/ShooterGame.PrimalDinoCharacter|GetBabyAge _array_element)) false)
              (Class|PrimalCharacterStatusComponent|RescaleAllStats _returnvalue)
              (Class|PrimalCharacterStatusComponent|ServerSyncReplicatedValues _returnvalue)
              (CallFunction|ForceUpdateImprintingEvent _array_element (Math|Float|Min(Float) _maximprint (Variables|/Script/ShooterGame.PrimalDinoCharacter|GetBabyAge _array_element)))
              (Class|PrimalBuff|StaticAddBuff "/Game/Mods/StructuresPlusMod/Misc/Nanny/Buff_NannyImprint.Buff_NannyImprint_C" _array_element 0 0 false))))))))

(fn HandleFeeding
  (params (Dinos :type Array%20of%20Primal%20Dino%20Character%20Object%20References))
  (bind (_inventoryfoodqty _consumedfoodarray) (Feeding|GetInventoryFoodQty))
  (if (> (Utilities|Array|Length _inventoryfoodqty) 0)
    (Feeding|UpdateDinoFoodList Dinos)
    (LocalVariables|SetConsumedFoodQty _consumedfoodarray)
    (for _array_element Dinos
      (Utilities|FlowControl|Sequence
        (:then_0
          (if (Variables|/Script/Engine.Actor|GetbStasised _array_element)
            (Class|Actor|Unstasis _array_element)
            (Class|PrimalInventoryComponent|InventoryRefresh (Variables|/Script/ShooterGame.PrimalCharacter|GetMyInventoryComponent _array_element))))
        (:then_1
          (bind _foods (Feeding|GetDinoFoods _array_element))
          (bind _hasfood (Feeding|DoesDinoHaveFoodAlready _array_element _foods))
          (if (not _hasfood)
            (CallFunction|FeedDino _array_element _foods _inventoryfoodqty (LocalVariables|GetConsumedFoodQty))))))
    (for _array_element_2 (LocalVariables|GetConsumedFoodQty)
      (if (> (Math|Float|Floor (.BaseResourceRequirement (Utilities|Struct|BreakCraftingResourceRequirement _array_element_2))) 0)
        (Class|PrimalInventoryComponent|BPIncrementItemTemplateQuantity (Variables|Default|GetMyInventoryComponent) (.ResourceItemType (Utilities|Struct|BreakCraftingResourceRequirement _array_element_2)) (* (Math|Float|Floor (.BaseResourceRequirement (Utilities|Struct|BreakCraftingResourceRequirement _array_element_2))) -1) true false true false false false 0 false)))))

(fn UpdateDinoFoodList
  (params (Dinos :type Array%20of%20Primal%20Dino%20Character%20Object%20References))
  (for _array_element Dinos
    (bind _asprimaldinocharacter (Utilities|Casting|CastToPrimalDinoCharacterClass (Utilities|GetClass _array_element)))
    (bind _contains (Feeding|DoesDinoFoodListContainDino _asprimaldinocharacter))
    (if (not _contains)
      (Feeding|AddDinotoDinoFoodList _array_element))))

(fn DoesDinoFoodListContainDino
  (params (DinoClass :type Primal%20Dino%20Character%20Class%20Reference))
  (bind _array_element (Utilities|Array|ForEachLoopwithBreak (Variables|Feeding|GetFoodList) :!label _label)
    (:LoopBody
      (if (== (Utilities|Struct|BreakSPDinoFood _array_element) DinoClass)
        (goto _label Break)))
    (:Completed
      (return (LocalVariables|GetFoodListContainsDino)))))

(fn AddDinotoDinoFoodList
  (params (Dino :type Primal%20Dino%20Character%20Object%20Reference))
  (bind _rawfoodentry (Feeding|CreateDinoFoodListEntry Dino))
  (bind _sortedentry (Feeding|SortDinoFoodListEntry _rawfoodentry))
  (Utilities|Array|Add (Variables|Feeding|GetFoodList) _sortedentry))

(fn CreateDinoFoodListEntry
  (params (Dino :type Primal%20Dino%20Character%20Object%20Reference))
  (bind _asprimaldinocharacter (Utilities|Casting|CastToPrimalDinoCharacterClass (Utilities|GetClass Dino)))
  (Utilities|Struct|SetmembersinSPDinoFood (LocalVariables|GetRawEntry) _asprimaldinocharacter)
  (Utilities|FlowControl|Sequence
    (:then_0
      (for _array_element (Variables|/Script/ShooterGame.PrimalDinoSettings|GetFoodEffectivenessMultipliers (Variables|/Script/ShooterGame.PrimalDinoCharacter|GetMyDinoSettingsCDO Dino))
        (if (Math|Boolean|ANDBoolean (> (.FoodEffectivenessMultiplier (Utilities|Struct|BreakDinoFoodEffectivenessMultipliers _array_element)) 0.0) (!= (.FoodItemParent (Utilities|Struct|BreakDinoFoodEffectivenessMultipliers _array_element)) "/Game/PrimalEarth/CoreBlueprints/Items/Consumables/PrimalItemConsumable_SuperTestMeat.PrimalItemConsumable_SuperTestMeat_C") (!= (.FoodItemParent (Utilities|Struct|BreakDinoFoodEffectivenessMultipliers _array_element)) "/Game/PrimalEarth/CoreBlueprints/Items/Consumables/PrimalItemConsumable_Kibble_Base.PrimalItemConsumable_Kibble_Base_C"))
          (bind _value (Feeding|GetFoodValue (.FoodItemParent (Utilities|Struct|BreakDinoFoodEffectivenessMultipliers _array_element)) (.FoodEffectivenessMultiplier (Utilities|Struct|BreakDinoFoodEffectivenessMultipliers _array_element))))
          (bind _newaffinity (Feeding|NormalizeAffinity (.FoodItemParent (Utilities|Struct|BreakDinoFoodEffectivenessMultipliers _array_element)) (.AffinityOverride (Utilities|Struct|BreakDinoFoodEffectivenessMultipliers _array_element))))
          (Utilities|Array|Add (Utilities|Struct|BreakSPDinoFood (LocalVariables|GetRawEntry)) (Utilities|Struct|MakeSPDinoFoodEntry (.FoodItemParent (Utilities|Struct|BreakDinoFoodEffectivenessMultipliers _array_element)) _value _newaffinity)))))
    (:then_1
      (return (LocalVariables|GetRawEntry)))))

(fn GetFoodValue
  (params (FoodClass :type Primal%20Item%20Class%20Reference) (Effectiveness :type Float%20%28single-precision%29))
  (bind _returnvalue (Class|VictoryCore|GetClassDefaultObject FoodClass))
  (bind _asprimalitem (Utilities|Casting|CastToPrimalItem _returnvalue))
  (bind _array_element (Utilities|Array|ForEachLoopwithBreak (Variables|/Script/ShooterGame.PrimalItem|GetUseItemAddCharacterStatusValues _asprimalitem) :!label _label)
    (:LoopBody
      (if (Utilities|Enum|Equal(Enum) (.StatusValueType (Utilities|Struct|BreakUseItemAddCharacterStatusValue _array_element)) "Food")
        (LocalVariables|SetActualFoodValue (* (.BaseAmountToAdd (Utilities|Struct|BreakUseItemAddCharacterStatusValue _array_element)) Effectiveness))
        (goto _label Break)))
    (:Completed
      (return (Math|Float|SelectFloat Effectiveness (LocalVariables|GetActualFoodValue) (== (LocalVariables|GetActualFoodValue) 0.0))))))

(fn SortDinoFoodListEntry
  (params (RawEntry :type SP%20Dino%20Food%20Structure))
  (bind (_dinoclass _foodlist) (Utilities|Struct|BreakSPDinoFood RawEntry))
  (bind _sortedfoodlist (LocalVariables|GetSortedFoodList))
  (while (and (> (Utilities|Array|Length _foodlist) 0) (< (LocalVariables|GetIter) 100))
    (LocalVariables|SetIter (+ (LocalVariables|GetIter) 1))
    (LocalVariables|SetLowestAffinity 999999999.0)
    (for (_array_element _array_index) _foodlist
      (if (< (Utilities|Struct|BreakSPDinoFoodEntry _array_element) (LocalVariables|GetLowestAffinity))
        (LocalVariables|SetLowestAffinity (Utilities|Struct|BreakSPDinoFoodEntry _array_element))
        (LocalVariables|SetLowestAffinityIndex _array_index)))
    (Utilities|Array|Add (LocalVariables|GetSortedFoodList) (Utilities|Struct|MakeSPDinoFoodEntry (.FoodClass (Utilities|Struct|BreakSPDinoFoodEntry (Utilities|Array|Get(acopy) _foodlist (LocalVariables|GetLowestAffinityIndex)))) (.FoodValue (Utilities|Struct|BreakSPDinoFoodEntry (Utilities|Array|Get(acopy) _foodlist (LocalVariables|GetLowestAffinityIndex)))) (.FoodAffinity (Utilities|Struct|BreakSPDinoFoodEntry (Utilities|Array|Get(acopy) _foodlist (LocalVariables|GetLowestAffinityIndex))))))
    (Utilities|Array|RemoveIndex _foodlist (LocalVariables|GetLowestAffinityIndex)))
  (Utilities|Array|Add _sortedfoodlist (Utilities|Struct|MakeSPDinoFoodEntry "/Game/PrimalEarth/CoreBlueprints/Items/Consumables/PrimalItemConsumable_Kibble_Base.PrimalItemConsumable_Kibble_Base_C" 6e+01 999.0))
  (return (Utilities|Struct|MakeSPDinoFood _dinoclass _sortedfoodlist)))

(fn NormalizeAffinity
  (params (FoodClass :type Primal%20Item%20Class%20Reference) (OriginalAffinity :type Float%20%28single-precision%29))
  (LocalVariables|SetAdjustedAffinity OriginalAffinity)
  (if (== FoodClass "/Game/PrimalEarth/CoreBlueprints/Items/Consumables/PrimalItemConsumable_SweetVeggieCake.PrimalItemConsumable_SweetVeggieCake_C")
    (LocalVariables|SetAdjustedAffinity 999.0)
    (else
      (return (LocalVariables|GetAdjustedAffinity)))))

(fn GetDinoFoods
  (params (Dino :type Primal%20Dino%20Character%20Object%20Reference))
  (bind _asprimaldinocharacter (Utilities|Casting|CastToPrimalDinoCharacterClass (Utilities|GetClass Dino)))
  (bind _array_element (Utilities|Array|ForEachLoopwithBreak (Variables|Feeding|GetFoodList) :!label _label)
    (:LoopBody
      (if (== (.DinoClass (Utilities|Struct|BreakSPDinoFood _array_element)) _asprimaldinocharacter)
        (LocalVariables|SetDinoFoods (.FoodList (Utilities|Struct|BreakSPDinoFood _array_element)))
        (goto _label Break)))
    (:Completed
      (return (LocalVariables|GetDinoFoods)))))

(fn FeedDino
  (params (Dino :type Primal%20Dino%20Character%20Object%20Reference) (Foods :type Array%20of%20SP%20Dino%20Food%20Entry%20Structures) (FoodInInventory :type Array%20of%20Crafting%20Resource%20Requirement%20Structures) (ConsumedFood :type Array%20of%20Crafting%20Resource%20Requirement%20Structures))
  (bind _returnvalue (Class|PrimalCharacter|GetCharacterStatusComponent Dino))
  (if (>= (* (Variables|Feeding|GetFeedingThreshold) 0.01) (/ (Class|PrimalCharacterStatusComponent|BPGetCurrentStatusValue _returnvalue "Food") (Class|PrimalCharacterStatusComponent|BPGetMaxStatusValue _returnvalue "Food")))
    (bind _array_element (Utilities|Array|ForEachLoopwithBreak Foods :!label _label)
      (:LoopBody
        (if (LocalVariables|GetFinishedFeeding)
          (goto _label Break)
          (else
            (bind (_array_element_2 _array_index) (Utilities|Array|ForEachLoopwithBreak FoodInInventory :!label _label_2)
              (:LoopBody
                (LocalVariables|SetCurrentTransferAmt 0)
                (if (Utilities|ClassIsChildOf (.ResourceItemType (Utilities|Struct|BreakCraftingResourceRequirement _array_element_2)) (Utilities|Struct|BreakSPDinoFoodEntry _array_element))
                  (if (> (- (.BaseResourceRequirement (Utilities|Struct|BreakCraftingResourceRequirement _array_element_2)) (Utilities|Struct|BreakCraftingResourceRequirement (Utilities|Array|Get(acopy) ConsumedFood _array_index))) 0.0)
                    (LocalVariables|SetCurrentTransferAmt (Math|Float|Floor (Math|Float|Min(Float) (- (.BaseResourceRequirement (Utilities|Struct|BreakCraftingResourceRequirement _array_element_2)) (Utilities|Struct|BreakCraftingResourceRequirement (Utilities|Array|Get(acopy) ConsumedFood _array_index))) (Math|Conversions|ToFloat(Integer) (Math|Integer|SelectInt 1 (- (Utilities|Array|Get(acopy) (Variables|Feeding|GetFoodTransferAmts) (Variables|Feeding|GetFoodTransferAmtIndex)) (LocalVariables|GetCurrentTransferTotal)) (== (Utilities|Struct|BreakSPDinoFoodEntry _array_element) "/Game/PrimalEarth/CoreBlueprints/Items/Consumables/BaseBPs/PrimalItemConsumable_WyvernMilk.PrimalItemConsumable_WyvernMilk_C"))))))
                    (Class|PrimalInventoryComponent|BPIncrementItemTemplateQuantity (Variables|/Script/ShooterGame.PrimalCharacter|GetMyInventoryComponent Dino) (.ResourceItemType (Utilities|Struct|BreakCraftingResourceRequirement _array_element_2)) (LocalVariables|GetCurrentTransferAmt) true false false false false false 0 false)
                    (Utilities|Array|SetArrayElem ConsumedFood _array_index (Utilities|Struct|MakeCraftingResourceRequirement (+ (Utilities|Struct|BreakCraftingResourceRequirement (Utilities|Array|Get(acopy) ConsumedFood _array_index)) (Math|Conversions|ToFloat(Integer) (LocalVariables|GetCurrentTransferAmt))) (.ResourceItemType (Utilities|Struct|BreakCraftingResourceRequirement _array_element_2))))
                    (LocalVariables|SetCurrentTransferTotal (+ (LocalVariables|GetCurrentTransferAmt) (LocalVariables|GetCurrentTransferTotal)))
                    (if (or (>= (LocalVariables|GetCurrentTransferTotal) (Utilities|Array|Get(acopy) (Variables|Feeding|GetFoodTransferAmts) (Variables|Feeding|GetFoodTransferAmtIndex))) (== (Utilities|Struct|BreakSPDinoFoodEntry _array_element) "/Game/PrimalEarth/CoreBlueprints/Items/Consumables/BaseBPs/PrimalItemConsumable_WyvernMilk.PrimalItemConsumable_WyvernMilk_C"))
                      (LocalVariables|SetFinishedFeeding true)
                      (goto _label_2 Break)))))))))
      (:Completed
        (if (> (LocalVariables|GetCurrentTransferTotal) 0)
          (Class|PrimalBuff|StaticAddBuff "/Game/Mods/StructuresPlusMod/Misc/Nanny/Buff_NannyFeed.Buff_NannyFeed_C" Dino 0 0 false))))))

(fn GetInventoryFoodQty
  (for _array_element (Variables|/Script/ShooterGame.PrimalInventoryComponent|GetInventoryItems (Variables|Default|GetMyInventoryComponent))
    (LocalVariables|SetFoundExistingFoodItem false)
    (bind _asprimalitem (Utilities|Casting|CastToPrimalItemClass (Utilities|GetClass _array_element)))
    (if (not (Utilities|ClassIsChildOf _asprimalitem "/Game/PrimalEarth/CoreBlueprints/Items/Consumables/PrimalItemConsumable_Honey.PrimalItemConsumable_Honey_C"))
      (bind (_array_element_2 _array_index) (Utilities|Array|ForEachLoopwithBreak (LocalVariables|GetInvFoodQtyTotals) :!label _label)
        (:LoopBody
          (if (== _asprimalitem (.ResourceItemType (Utilities|Struct|BreakCraftingResourceRequirement _array_element_2)))
            (LocalVariables|SetFoundExistingFoodItem true)
            (Utilities|Array|SetArrayElem (LocalVariables|GetInvFoodQtyTotals) _array_index (Utilities|Struct|MakeCraftingResourceRequirement (+ (.BaseResourceRequirement (Utilities|Struct|BreakCraftingResourceRequirement _array_element_2)) (Math|Conversions|ToFloat(Integer) (Variables|/Script/ShooterGame.PrimalItem|GetItemQuantity _array_element))) (.ResourceItemType (Utilities|Struct|BreakCraftingResourceRequirement _array_element_2))))
            (goto _label Break)))
        (:Completed
          (if (not (LocalVariables|GetFoundExistingFoodItem))
            (Utilities|Array|Add (LocalVariables|GetInvFoodQtyTotals) (Utilities|Struct|MakeCraftingResourceRequirement (Math|Conversions|ToFloat(Integer) (Variables|/Script/ShooterGame.PrimalItem|GetItemQuantity _array_element)) _asprimalitem))
            (Utilities|Array|Add (LocalVariables|GetInvFoodConsumedArray) (Utilities|Struct|MakeCraftingResourceRequirement _asprimalitem)))))))
  (return (LocalVariables|GetInvFoodQtyTotals) (LocalVariables|GetInvFoodConsumedArray)))

(fn DoesDinoHaveFoodAlready
  (params (Dino :type Primal%20Dino%20Character%20Object%20Reference) (Foods :type Array%20of%20SP%20Dino%20Food%20Entry%20Structures))
  (bind _array_element (Utilities|Array|ForEachLoopwithBreak (Variables|/Script/ShooterGame.PrimalInventoryComponent|GetInventoryItems (Variables|/Script/ShooterGame.PrimalCharacter|GetMyInventoryComponent Dino)) :!label _label)
    (:LoopBody
      (if (not (Variables|/Script/ShooterGame.PrimalItem|GetbIsBlueprint _array_element))
        (if (LocalVariables|GetHasFoodInInventory)
          (goto _label Break)
          (else
            (bind _array_element_2 (Utilities|Array|ForEachLoopwithBreak Foods :!label _label_2)
              (:LoopBody
                (if (Utilities|ClassIsChildOf (Utilities|GetClass _array_element) (Utilities|Struct|BreakSPDinoFoodEntry _array_element_2))
                  (LocalVariables|SetHasFoodInInventory true)
                  (goto _label_2 Break))))))))
    (:Completed
      (return (LocalVariables|GetHasFoodInInventory)))))

(fn BPClientDoMultiUse
  (params (ForPC :type Player%20Controller%20Object%20Reference) (ClientUseIndex :type Integer))
  (bind _asshooterplayercontroller (Utilities|Casting|CastToShooterPlayerController ForPC))
  (if (== ClientUseIndex 9003)
    (Class|ShooterPlayerController|SetMultiUseWheelCategory _asshooterplayercontroller 1)))

(fn ReceiveBeginPlay
  (bind _returnvalue (Game|GetGameMode))
  (|CallParentFunction)
  (if (not (Variables|Default|GetbIsPreviewStructure))
    (Networking|SwitchHasAuthority
      (:Authority
        (Utilities|FlowControl|Sequence
          (:then_0
            (bind _value (CallFunction|SPGetConfigSetting-InventorySize _returnvalue "NannySlotCount" 100))
            (Variables|Default|SetInvSlotOverride _value true))
          (:then_1
            (bind _value_2 (CallFunction|SPGetConfig-Int _returnvalue "NannyRangeInFoundations" 10 1 50))
            (Variables|Default|SetScanRadius (* _value_2 3e+02) true))
          (:then_2
            (bind _value_3 (CallFunction|SPGetConfig-Float _returnvalue "NannyMaxImprint" 1e+02 1.0 1e+02))
            (Variables|Imprinting|SetMaxImprint (/ _value_3 1e+02)))
          (:then_3
            (bind _value_4 (CallFunction|SPGetConfig-Bool _returnvalue "DisableNannyImprinting"))
            (Variables|Imprinting|SetDisableNannyImprinting _value_4))
          (:then_4
            (bind _value_5 (CallFunction|SPGetConfig-Float _returnvalue "NannyIntervalInSeconds" 35.0 5.0 1.8e+03))
            (Variables|Default|SetScanInterval _value_5))
          (:then_5
            (bind _value_6 (CallFunction|SPGetConfig-Int _returnvalue "NannyFeedingStartThreshold" 20 1 100))
            (Variables|Feeding|SetFeedingThreshold _value_6)))))))

(fn BPGetMultiUseEntries
  (params (ForPC :type Player%20Controller%20Object%20Reference) (MultiUseEntries :type Array%20of%20Multi%20Use%20Entry%20Structures))
  (bind _color (CallFunction|SPGetMultiUseSpecialColor))
  (bind _returnvalue (Math|Conversions|ToColor(LinearColor) _color))
  (bind _returnvalue_2 (|CallParentFunction ForPC MultiUseEntries))
  (Utilities|FlowControl|Sequence
    (:then_0
      (bind _returnvalue_3 (Class|PrimalStructure|AllowStructureAccess ForPC))
      (if _returnvalue_3
        (Utilities|Array|Add _returnvalue_2 (Utilities|Struct|MakeMultiUseEntry "[Change Food Amt]" 9003 -1010 true true _returnvalue))
        (Utilities|Array|Add _returnvalue_2 (Utilities|Struct|MakeMultiUseEntry "Transfers this amount every time a dino needs food" 8999 5000 true true 1 (Math|Color|MakeColor 255 255 255 255)))
        (for (_array_element _array_index) (Variables|Feeding|GetFoodTransferAmts)
          (Utilities|Array|Add _returnvalue_2 (Utilities|Struct|MakeMultiUseEntry (Utilities|String|ToString(Integer) _array_element) (+ _array_index 9010) (* _array_index -1) (== _array_index (Variables|Feeding|GetFoodTransferAmtIndex)) 1 _returnvalue)))
        (if (not (Variables|Imprinting|GetDisableNannyImprinting))
          (Utilities|Array|Add _returnvalue_2 (Utilities|Struct|MakeMultiUseEntry (Utilities|String|SelectString "Enable Imprinting" "Disable Imprinting" (Variables|Imprinting|GetDisableImprinting)) 9004 -1011)))))
    (:then_1
      (return _returnvalue_2))))

(fn BPTryMultiUse
  (params (ForPC :type Player%20Controller%20Object%20Reference) (UseIndex :type Integer))
  (bind _returnvalue (Class|KismetSystemLibrary|MakeLiteralInteger 9010))
  (|CallParentFunction ForPC UseIndex)
  (Utilities|FlowControl|Sequence
    (:then_0
      (if (== UseIndex 9004)
        (Variables|Imprinting|SetDisableImprinting (not (Variables|Imprinting|GetDisableImprinting)) true)
        (elif (and (>= UseIndex _returnvalue) (< UseIndex (+ _returnvalue (Utilities|Array|Length (Variables|Feeding|GetFoodTransferAmts)))))
          (Variables|Feeding|SetFoodTransferAmtIndex (- UseIndex _returnvalue) true))))
    (:then_1
      (return true))))

(fn DoScan
  (if (Variables|Default|GetbContainerActivated)
    (CallFunction|HandleImprinting (Variables|Imprinting|GetImprintingDinoList))
    (Class|PrimalInventoryComponent|InventoryRefresh (Variables|Default|GetMyInventoryComponent))
    (bind (_feedlist _imprintlist) (CallFunction|GetDinos))
    (Utilities|FlowControl|Sequence
      (:then_0
        (CallFunction|HandleFeeding _feedlist))
      (:then_1
        (if (and (not (Variables|Imprinting|GetDisableNannyImprinting)) (not (Variables|Imprinting|GetDisableImprinting)))
          (Variables|Imprinting|SetImprintingDinoList _imprintlist)))
      (:then_2
        (Utilities|Time|SetTimerbyFunctionName 0 "DoScan" (CallFunction|GetScanInterval))))))